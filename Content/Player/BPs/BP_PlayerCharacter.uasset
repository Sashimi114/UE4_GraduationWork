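; Player character for a two-player robot fighting game, tagged Player 01 or 02 to set its texture and opponent.
; Input events check state flags, then trigger GAS abilities for attacks, air combos, specials and dodges, while guard locks facing and camera yaw tracks the opponent.
; Weapon overlaps and beam traces apply damage through a gate that closes for avoidance and flashing invincibility.
; Damage drives hit stop, knockback, launches, downs and slow-motion KO ending the match.
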(event OnComponentBeginOverlap(ECollision)
  (params (OverlappedComponent :type Primitive%20Component%20Object%20Reference) (OtherActor :type Actor%20Object%20Reference) (OtherComp :type Primitive%20Component%20Object%20Reference) (OtherBodyIndex :type Integer) (bFromSweep :type Boolean) (SweepResult :type Hit%20Result%20Structure%20%28by%20ref%29))
  (bind _opponentplayercontrollerid (Variables|PlayerControllerID|GetOpponentPlayerControllerID))
  (bind _returnvalue (Game|GetPlayerController _opponentplayercontrollerid))
  (if (CallFunction|IsActorCheck OtherActor)
    (Transformation|SetActorRotation OtherActor (Math|Rotator|MakeRotator 0.0 0.0 (.Yaw (Math|Rotator|BreakRotator (Math|Rotator|FindLookatRotation (Transformation|GetActorLocation) (Transformation|GetActorLocation))))))
    (Class|BPPlayerConInterface|IsinInputPossible?(Message) _returnvalue false)
    (Utilities|FlowControl|Delay 1.0)
    (Class|BPPlayerConInterface|IsinInputPossible?(Message) _returnvalue true)))

(event OnComponentBeginOverlap(AttackCollision)
  (params (OverlappedComponent :type Primitive%20Component%20Object%20Reference) (OtherActor :type Actor%20Object%20Reference) (OtherComp :type Primitive%20Component%20Object%20Reference) (OtherBodyIndex :type Integer) (bFromSweep :type Boolean) (SweepResult :type Hit%20Result%20Structure%20%28by%20ref%29))
  (bind _characterref (Variables|Actor|GetCharacterRef))
  ;[0 0.9531 1] ダメージ判定
  (if (CallFunction|IsActorCheck OtherActor)
    (if (Variables|BP_PlayerCharacter_C|GetIs%20In%20Guard%20？ _characterref)
      (Transformation|AddActorLocalOffset (Variables|Actor|GetCharacterRef) (Math|Vector|MakeVector (Variables|BP_PlayerCharacter_C|GetGuard%20Back (Variables|Actor|GetCharacterRef)) 0.0 0.0) true true)
      (Niagara|SpawnSystematLocation "/Game/Player/Effect/Niagara/NS_GuardHit.NS_GuardHit" (Transformation|GetSocketLocation (Variables|/Script/Engine.Character|GetMesh (Variables|Actor|GetCharacterRef)) "HitE"))
      (elif (Math|Boolean|Equal(Boolean) (Variables|BP_PlayerCharacter_C|GetCheckFlame _characterref) (Variables|Default|GetCheckFlame))
        (CallFunction|FinishDamage)
        (Niagara|SpawnSystematLocation "/Game/sA_Megapack_v1/sA_Rayvfx/Fx/NiagaraSystems/NS_Energy_2.NS_Energy_2" (+ (Transformation|GetActorForwardVector) (Transformation|GetActorForwardVector (Variables|Actor|GetCharacterRef))) "0, 0, 0" "1.000000,0.200000,0.200000")
        (else
          (GameplayEffects|ApplyGameplayEffectToSelf :self (Variables|Default|GetAbilitySystem) :GameplayEffectClass "/Game/Player/GameplayEffect/GPE_DeadlyRecovery_Attack.GPE_DeadlyRecovery_Attack_C" :Level 1.0)
          (Game|Damage|ApplyDamage (Variables|Actor|GetCharacterRef) (Variables|Comboステータス|GetDamage) 0 0))))))

(event Custom|Finish%20Damage
  ;[0.3828 1 0] 武器の判定制御
  (Collision|SetCollisionEnabled (Variables|Collision|GetAttack%20Collision) "NoCollision"))

(event Custom|DeadlyShot
  (bind _mesh (Variables|Character|GetMesh))
  (bind _returnvalue (Transformation|GetSocketLocation _mesh "Launcher"))
  (bind _returnvalue_2 (Transformation|GetWorldRotation _mesh))
  ;[0 1 0.2031] 必殺
  (Variables|IsIn~|SetIs%20In%20LookON%20? false)
  (Audio|PlaySound2D "/Game/Player/Sound/S_Deadly.S_Deadly" 1.0 1.0 0.0 0 0)
  (bind _returnvalue_3 (Niagara|SpawnSystematLocation "/Game/sA_Megapack_v1/sA_Rayvfx/Fx/NiagaraSystems/NS_Ray_1.NS_Ray_1" _returnvalue (Transformation|GetSocketRotation _mesh "Launcher") "1.000000,0.200000,0.200000"))
  (Variables|Default|SetNewVar_0 _returnvalue_3)
  (bind _outhit (Collision|LineTraceByChannel _returnvalue (+ _returnvalue (* (Math|Vector|GetForwardVector (Math|Rotator|MakeRotator (.roll _returnvalue_2) (.pitch _returnvalue_2) (+ (.yaw _returnvalue_2) 9e+01))) 1e+03)) "TraceTypeQuery2" true 0 "None" false "(R=1.000000,G=0.000000,B=0.000000,A=1.000000)" "(R=0.000000,G=1.000000,B=0.000000,A=1.000000)" 2.0))
  (if (== (.HitActor (Collision|BreakHitResult _outhit)) (Variables|Actor|GetCharacterRef))
    (Game|Damage|ApplyDamage (.HitActor (Collision|BreakHitResult _outhit)) (Variables|Comboステータス|GetDamage) 0 0)))

(event Custom|EndAvoidance
  ;[1 0.2109 0] 回避
  ;;[0 0.2969 1] 回避の判定制御
  (CallFunction|Open))

(event Custom|StartAvoidance
  ;[1 0.2109 0] 回避
  ;;[0 0.2969 1] 回避の判定制御
  (CallFunction|Close))

(event Custom|Open
  (bind _mesh (Variables|Character|GetMesh))
  (bind _mesh_2 (Variables|Character|GetMesh))
  (bind _returnvalue (Transformation|GetSocketLocation _mesh "HitE"))
  (bind _returnvalue_2 (Transformation|GetSocketLocation _mesh_2 "HitE"))
  ;[1 0 0.9609] ダメージ処理
  (Utilities|FlowControl|Gate false) ; enters at Open
)

(event Custom|Off%20FlameCheck
  ;[0 0.9531 1] ダメージ判定
  (Variables|Default|SetCheckFlame false))

(event Custom|On%20FlameCheck
  ;[0 0.9531 1] ダメージ判定
  (Variables|Default|SetCheckFlame true))

(event Custom|Start%20Damage
  ;[0.3828 1 0] 武器の判定制御
  (Collision|SetCollisionEnabled (Variables|Collision|GetAttack%20Collision) "QueryOnly"))

(event Custom|Close
  (bind _mesh (Variables|Character|GetMesh))
  (bind _mesh_2 (Variables|Character|GetMesh))
  (bind _returnvalue (Transformation|GetSocketLocation _mesh "HitE"))
  (bind _returnvalue_2 (Transformation|GetSocketLocation _mesh_2 "HitE"))
  ;[1 0 0.9609] ダメージ処理
  (Utilities|FlowControl|Gate false) ; enters at Close
)

(event EventBeginPlay
  ;[0.07812 1 0] 初期化
  (Utilities|FlowControl|Sequence
    (:then_0
      (Collision|SetCollisionEnabled (Variables|Collision|GetAttack%20Collision) "NoCollision")
      (Collision|SetCollisionEnabled (Variables|Default|GetECollision) "NoCollision")
      (Variables|Default|SetAnim%20Enum%20Value 0))
    (:then_1
      (bind _returnvalue (Rendering|Material|CreateDynamicMaterialInstance "/Game/Player/Model/robot/lambert1_Inst.lambert1_Inst" "None" "None" :!class /Script/Engine.KismetMaterialLibrary))
      (bind _output_get (Variables|Material|SetPlayerMaterial%200 _returnvalue))
      (Rendering|Material|SetMaterial (Variables|Character|GetMesh) 0 _output_get))))

(event EventSetCharacterRef
  (bind _self self)
  (bind _opponentplayercontrollerid (Variables|PlayerControllerID|GetOpponentPlayerControllerID))
  ;[0.5938 0 1] 相手Playerを取得
  (switch name (Utilities|Array|Get(acopy) (Variables|Default|GetTags))
    (:Player01
      (bind _asbp_player_character (Utilities|Casting|CastToBP_PlayerCharacter (Game|GetPlayerCharacter _opponentplayercontrollerid)))
      (Variables|BP_PlayerCharacter_C|SetCharacterRef _self _asbp_player_character))
    (:Player02
      (bind _asbp_player_character_2 (Utilities|Casting|CastToBP_PlayerCharacter (Game|GetPlayerCharacter _opponentplayercontrollerid)))
      (Variables|BP_PlayerCharacter_C|SetCharacterRef _self _asbp_player_character_2))))

(event EventDeadlyEvent
  ;[0 1 0.2031] 必殺
  (if (not (Math|Boolean|ORBoolean (Variables|Isin~|GetIs%20In%20Damage%20?) (Variables|IsIn~|GetIs%20In%20Guard%20？) (Variables|IsIn~|GetIs%20In%20Down?)))
    (Abilities|TryActivateAbilitiesbyTag (Variables|Default|GetAbilitySystem) (Utilities|Struct|MakeGameplayTagContainer (Utilities|Array|MakeArray "(TagName=\"Ability.Action.Deadly\")")) true)))

(event EventJumpStopEvent
  ;[0 1 0.8359] ジャンプ
  (Character|StopJumping)
  (Variables|IsIn~|SetIs%20In%20Jump? false))

(event EventJumpEvent
  ;[0 1 0.8359] ジャンプ
  (if (not (Math|Boolean|ORBoolean (Variables|Isin~|GetIs%20In%20Damage%20?) (Variables|IsIn~|GetIs%20In%20Deadly%20?) (Variables|IsIn~|GetIs%20In%20Guard%20？) (Variables|IsIn~|GetIs%20In%20Attack?)))
    (Character|Jump)
    (Variables|IsIn~|SetIs%20In%20Jump? true)))

(event EventOFFGuard
  ;[1 0 0.75] ガード
  (Variables|IsIn~|SetIs%20In%20Guard%20？ false)
  (Variables|IsIn~|SetIs%20In%20LookON%20? false))

(event EventOnGuard
  ;[1 0 0.75] ガード
  (if (not (Math|Boolean|ORBoolean (Variables|Isin~|GetIs%20In%20Damage%20?) (Variables|IsIn~|GetIs%20In%20Deadly%20?) (Variables|IsIn~|GetIs%20In%20Down?)))
    (if (not (AI|Components|NavMovement|IsFalling (Variables|Character|GetCharacterMovement)))
      (Transformation|SetActorRotation (Math|Rotator|MakeRotator 0.0 0.0 (.Z (CallFunction|GetPlayerFindLookatRotation (Variables|PlayerControllerID|GetOpponentPlayerControllerID)))))
      (Variables|IsIn~|SetIs%20In%20Guard%20？ true)
      (Variables|IsIn~|SetIs%20In%20LookON%20? true))))

(event EventMoveCollision
  (bind _attack_collision (Variables|Collision|GetAttack%20Collision))
  ;[0.3828 1 0] 武器の判定制御
  (Transformation|SetWorldLocation (Variables|Collision|GetAttack%20Collision) (+ (Transformation|GetWorldLocation _attack_collision) (* (Math|Vector|GetRightVector _attack_collision) (Variables|Comboステータス|GetMoveCollisionVec))) false false))

(event EventHeavyAttack
  (bind _opponentplayercontrollerid (Variables|PlayerControllerID|GetOpponentPlayerControllerID))
  ;[1 0 0] 攻撃
  ;;[0.3594 1 0] 強攻撃
  (if (not (Math|Boolean|ORBoolean (Variables|Isin~|GetIs%20In%20Damage%20?) (Variables|IsIn~|GetIs%20In%20Deadly%20?) (Variables|IsIn~|GetIs%20In%20Down?)))
    (if (not (AI|Components|NavMovement|IsFalling (Variables|Character|GetCharacterMovement)))
      (Variables|IsIn~|SetIs%20In%20Attack? true)
      (if (CallFunction|IsDistancetoCheck _opponentplayercontrollerid)
        (Transformation|SetActorRotation (Math|Rotator|MakeRotator 0.0 0.0 (.Z (CallFunction|GetPlayerFindLookatRotation _opponentplayercontrollerid)))))
      (Abilities|TryActivateAbilitiesbyTag (Variables|Default|GetAbilitySystem) (Utilities|Struct|MakeGameplayTagContainer (Utilities|Array|MakeArray "(TagName=\"Ability.Action.UpAttack\")")) true))))

(event EventTick
  (params (DeltaSeconds :type Float%20%28single-precision%29))
  ;[0 0.5547 1] Update処理
  (Utilities|FlowControl|Sequence
    (:then_0
      (CallFunction|CameraMovement)
      (if (not (Variables|IsIn~|GetIs%20In%20Invincible?))
        (Rendering|Material|SetScalarParameterValue (Variables|Material|GetPlayerMaterial%200) "Mask" (Math|Float|MapRangeClamped (Math|Vector|Distance(Vector) (Transformation|GetWorldLocation (Variables|Default|GetFollowCamera)) (Transformation|GetActorLocation)) 1e+02 1.5e+02 0.1 1.0) :!class /Script/Engine.MaterialInstanceDynamic)))
    (:then_1
      (if (not (AI|Components|NavMovement|IsFalling (Variables|Character|GetCharacterMovement)))
        (bind _returnvalue (GameplayEffects|ApplyGameplayEffectToSelf :self (Variables|Default|GetAbilitySystem) :GameplayEffectClass "/Game/Player/GameplayEffect/GPE_RefreshSkyComboCount.GPE_RefreshSkyComboCount_C" :Level 1.0))
        (Variables|Default|SetRefreshSkyComboCountHandle _returnvalue)))
    (:then_2
      (if (Variables|IsIn~|GetIs%20In%20LookON%20?)
        (Transformation|SetActorRotation (Math|Rotator|MakeRotator 0.0 0.0 (.Z (CallFunction|GetPlayerFindLookatRotation (Variables|PlayerControllerID|GetOpponentPlayerControllerID)))))))))

(event Game|Damage|EventAnyDamage
  (params (Damage :type Float%20%28single-precision%29) (DamageType :type Damage%20Type%20Object%20Reference) (InstigatedBy :type Controller%20Object%20Reference) (DamageCauser :type Actor%20Object%20Reference))
  (bind _mesh (Variables|Character|GetMesh))
  (bind _mesh_2 (Variables|Character|GetMesh))
  (bind _returnvalue (Transformation|GetSocketLocation _mesh "HitE"))
  (bind _returnvalue_2 (Transformation|GetSocketLocation _mesh_2 "HitE"))
  ;[1 0 0.9609] ダメージ処理
  (Utilities|FlowControl|Gate false
    (:Exit
      (Transformation|SetActorRotation (Math|Rotator|MakeRotator 0.0 0.0 (.Z (CallFunction|GetPlayerFindLookatRotation (Variables|PlayerControllerID|GetOpponentPlayerControllerID)))))
      (Variables|Isin~|SetIs%20In%20Damage%20? true)
      (Variables|ステータス|SetHealth (- (Variables|ステータス|GetHealth) Damage))
      (CallFunction|Close)
      (if (CallFunction|IsAlive?)
        (Niagara|SpawnSystematLocation "/Game/Player/Effect/Niagara/NS_DamageHit.NS_DamageHit" _returnvalue_2)
        (Animation|StopAnimMontage "/Game/Player/Animation/AnimationMontage/robot/AM_Damage.AM_Damage")
        (Variables|Default|SetAnim%20Enum%20Value 1)
        (Variables|IsIn~|SetIs%20In%20Down? true)
        (Class|BPPlayerConInterface|IsinInputPossible?(Message) (Game|GetPlayerController (Variables|PlayerControllerID|GetOpponentPlayerControllerID)) false)
        (Class|BPPlayerConInterface|IsinInputPossible?(Message) (Game|GetPlayerController (Variables|PlayerControllerID|GetPlayerControllerID)) false)
        (Audio|PlaySound2D "/Game/Player/Sound/S_K_O.S_K_O" 1.0 1.0 0.0 0 0)
        (Utilities|Time|SetGlobalTimeDilation 0.4)
        (Utilities|FlowControl|Delay 2.0)
        (Utilities|Time|SetGlobalTimeDilation 1.0)
        (Default|Finish (.AsBP%20Match%20Game (Utilities|Casting|CastToBP_MatchGame (Game|GetGameMode))))
        (else
          (GameplayEffects|ApplyGameplayEffectToSelf :self (Variables|Default|GetAbilitySystem) :GameplayEffectClass "/Game/Player/GameplayEffect/GPE_DeadlyRecovery_Damage.GPE_DeadlyRecovery_Damage_C" :Level 1.0)
          (if (Variables|IsIn~|GetIs%20In%20Down?)
            (Niagara|SpawnSystematLocation "/Game/Player/Effect/Niagara/NS_DamageHit.NS_DamageHit" _returnvalue_2)
            (Utilities|HitStop (Variables|HitStop|GetHit%20Stop%20Time%20Dilation) self (Variables|Actor|GetCharacterRef) (Variables|PlayerControllerID|GetPlayerControllerID) (Variables|HitStop|GetHit%20Stop%20Duration)
              (:%20
                (Audio|PlaySound2D "/Game/Player/Sound/S_AttackHit3.S_AttackHit3" 1.0 1.0 0.0 0 0)
                (CallFunction|Open)))
            (elif (Variables|BP_PlayerCharacter_C|GetDownAttack (Variables|Actor|GetCharacterRef))
              (Animation|StopAnimMontage "/Game/Player/Animation/AnimationMontage/robot/AM_Damage.AM_Damage")
              (Variables|Default|SetAnim%20Enum%20Value 1)
              (Variables|IsIn~|SetIs%20In%20Down? true)
              (Niagara|SpawnSystematLocation "/Game/Player/Effect/Niagara/NS_DamageHit.NS_DamageHit" _returnvalue)
              (Utilities|HitStop (Variables|HitStop|GetHit%20Stop%20Time%20Dilation) self (Variables|Actor|GetCharacterRef) (Variables|PlayerControllerID|GetPlayerControllerID) (Variables|HitStop|GetHit%20Stop%20Duration)
                (:%20
                  (Audio|PlaySound2D "/Game/Player/Sound/S_AttackHit2.S_AttackHit2" 1.0 1.0 0.0 0 0)
                  (CallFunction|Open)
                  (Utilities|FlowControl|Delay 1.0)
                  (if (not (CallFunction|IsAlive?))
                    (Variables|IsIn~|SetIs%20In%20Down? false)
                    (Default|InvincibleTime self))))
              (else
                (Animation|Montage|PlayMontage (Variables|Character|GetMesh) "/Game/Player/Animation/AnimationMontage/robot/AM_Damage.AM_Damage"
                  (:then
                    (Niagara|SpawnSystematLocation "/Game/Player/Effect/Niagara/NS_DamageHit.NS_DamageHit" _returnvalue)
                    (Utilities|HitStop (Variables|HitStop|GetHit%20Stop%20Time%20Dilation) self (Variables|Actor|GetCharacterRef) (Variables|PlayerControllerID|GetPlayerControllerID) (Variables|HitStop|GetHit%20Stop%20Duration)
                      (:%20
                        (if (Variables|BP_PlayerCharacter_C|GetPounding%20Attack (Variables|Actor|GetCharacterRef))
                          (Animation|StopAnimMontage "/Game/Player/Animation/AnimationMontage/robot/AM_Damage.AM_Damage")
                          (Variables|IsIn~|SetIs%20In%20Down? true)
                          (Variables|Default|SetAnim%20Enum%20Value 1)
                          (Audio|PlaySound2D "/Game/Player/Sound/S_AttackHit2.S_AttackHit2" 1.0 1.0 0.0 0 0)
                          (Variables|Default|SetIniLocation (Transformation|GetActorLocation))
                          (bind _新規track_0 (Timeline|ActorUpVectorTime PlayFromStart)
                            (:Update
                              (Transformation|SetActorLocation (+ (* (Transformation|GetActorUpVector) (* _新規track_0 1e+01)) (Variables|Default|GetIniLocation)) false false))
                            (:Finished
                              (Variables|/Script/Engine.MovementComponent|SetVelocity (Variables|Character|GetCharacterMovement) "0, 0,-5.000000")
                              (CallFunction|Open)
                              (Utilities|FlowControl|Delay 1.0)
                              (if (not (CallFunction|IsAlive?))
                                (Variables|IsIn~|SetIs%20In%20Down? false)
                                (Default|InvincibleTime self))))
                          (else
                            (Transformation|AddActorLocalOffset (Math|Vector|MakeVector (Variables|BP_PlayerCharacter_C|GetStep%20Back (Variables|Actor|GetCharacterRef)) 0.0 0.0) true true)
                            (Audio|PlaySound2D "/Game/Player/Sound/S_AttackHit3.S_AttackHit3" 1.0 1.0 0.0 0 0)
                            (CallFunction|Open)
                            (Utilities|FlowControl|Delay 0.5)
                            (Variables|Isin~|SetIs%20In%20Damage%20? false)))))))))))))))

(event EventPressedAttack
  (bind _charactermovement (Variables|Character|GetCharacterMovement))
  (bind _opponentplayercontrollerid (Variables|PlayerControllerID|GetOpponentPlayerControllerID))
  ;[1 0 0] 攻撃
  (if (not (Math|Boolean|ORBoolean (Variables|Isin~|GetIs%20In%20Damage%20?) (Variables|IsIn~|GetIs%20In%20Deadly%20?) (Variables|IsIn~|GetIs%20In%20Down?)))
    (Variables|IsIn~|SetIs%20In%20Attack? true)
    (if (not (AI|Components|NavMovement|IsFalling (Variables|Character|GetCharacterMovement)))
      (Variables|IsIn~|SetIs%20In%20Attack? true)
      (if (CallFunction|IsDistancetoCheck _opponentplayercontrollerid)
        (Transformation|SetActorRotation (Math|Rotator|MakeRotator 0.0 0.0 (.Z (CallFunction|GetPlayerFindLookatRotation _opponentplayercontrollerid)))))
      ;;[0 0.002089 1] コンボ攻撃
      (Abilities|TryActivateAbilitiesbyTag (Variables|Default|GetAbilitySystem) (Utilities|Struct|MakeGameplayTagContainer (Utilities|Array|MakeArray "(TagName=\"Ability.Action.Attack\")")) true)
      (elif (> (Class|CharacterBase|GetSkyComboCount) 0.0)
        (Variables|IsIn~|SetIs%20In%20Attack? true)
        ;;[0 0.002089 1] 空中コンボ攻撃
        (Variables|/Script/Engine.CharacterMovementComponent|SetGravityScale _charactermovement 0.0)
        (Variables|/Script/Engine.MovementComponent|SetVelocity _charactermovement "0, 0, 0")
        (Abilities|TryActivateAbilitiesbyTag (Variables|Default|GetAbilitySystem) (Utilities|Struct|MakeGameplayTagContainer (Utilities|Array|MakeArray "(TagName=\"Ability.Action.SkyAttack\")")) true)
        (Utilities|FlowControl|Delay 0.7)
        (Default|ResetGravityScale self)))))

(event EventAvoid
  ;[1 0.2109 0] 回避
  (if (not (Math|Boolean|ORBoolean (Variables|Isin~|GetIs%20In%20Damage%20?) (Variables|IsIn~|GetIs%20In%20Guard%20？) (Variables|IsIn~|GetIs%20In%20Deadly%20?) (Variables|IsIn~|GetIs%20In%20Down?)))
    (Abilities|TryActivateAbilitybyClass (Variables|Default|GetAbilitySystem) "/Game/Player/GameplayAbility/GPA_Avoidance.GPA_Avoidance_C" true)))

(event EventSetControllerID
  (bind _playermaterial_0 (Variables|Material|GetPlayerMaterial%200))
  ;[0.4766 0 1] ControllerID取得
  (switch name (Utilities|Array|Get(acopy) (Variables|Default|GetTags))
    (:Player01
      (Variables|PlayerControllerID|SetOpponentPlayerControllerID 1)
      (Variables|PlayerControllerID|SetPlayerControllerID 0)
      (Rendering|Material|SetTextureParameterValue _playermaterial_0 "Texture" "/Game/Player/Model/robot/robot_texture/robot__BaseColor_red.robot__BaseColor_red"))
    (:Player02
      (Variables|PlayerControllerID|SetOpponentPlayerControllerID 0)
      (Variables|PlayerControllerID|SetPlayerControllerID 1)
      (Rendering|Material|SetTextureParameterValue _playermaterial_0 "Texture" "/Game/Player/Model/robot/robot_texture/robot_uv_lambert1_BaseColor.robot_uv_lambert1_BaseColor"))))

(event EventResetGravityScale
  ;[1 0.04688 0] 重力リセット
  (Variables|/Script/Engine.CharacterMovementComponent|SetGravityScale (Variables|Character|GetCharacterMovement) 1.0))

(event EventInvincibleTime
  ;[1 0 0.9609] ダメージ処理
  ;;[1 0.7734 0] 無敵時間
  (Variables|IsIn~|SetIs%20In%20Invincible? true)
  (CallFunction|Close)
  (Variables|Isin~|SetIs%20In%20Damage%20? false)
  (bind _flashingtime (Timeline|FlashingMaterialTime PlayFromStart)
    (:Update
      (Rendering|Material|SetScalarParameterValue (Variables|Material|GetPlayerMaterial%200) "Mask" _flashingtime :!class /Script/Engine.MaterialInstanceDynamic))
    (:Finished
      (CallFunction|Open)
      (Variables|Default|SetAnim%20Enum%20Value 0)
      (Variables|IsIn~|SetIs%20In%20Invincible? false))))

(event Input|ActionEvents|InputActionEmergencyAvoidance
  (params (Key :type Key%20Structure :default "None"))
  ;[1 0.6094 0] 緊急回避
  (:Pressed
    (if (not (Variables|IsIn~|GetIs%20In%20Down?))
      (Abilities|TryActivateAbilitiesbyTag (Variables|Default|GetAbilitySystem) (Utilities|Struct|MakeGameplayTagContainer (Utilities|Array|MakeArray "(TagName=\"Ability.Action.EmergencyAvoidance\")")) true))))

(fn ConstructionScript)

(fn CameraMovement
  (bind _opponentplayercontrollerid (Variables|PlayerControllerID|GetOpponentPlayerControllerID))
  (Utilities|FlowControl|Sequence
    (:then_0
      (if (not (CallFunction|CameraRange _opponentplayercontrollerid))
        (Pawn|Input|AddControllerYawInput (* (.Yaw (CallFunction|FindLookatRotationCamera (Game|GetPlayerCharacter _opponentplayercontrollerid))) 0.03))))))

(fn FindLookatRotationCamera
  (params (TagetActor :type Actor%20Object%20Reference))
  (bind _returnvalue (Transformation|GetActorLocation TagetActor))
  (bind _returnvalue_2 (Transformation|GetActorLocation))
  (bind _returnvalue_3 (Pawn|GetControlRotation :!class /Script/Engine.Pawn))
  (bind _returnvalue_4 (Math|Rotator|FindLookatRotation _returnvalue_2 (Math|Vector|MakeVector (.x _returnvalue) (.y _returnvalue) (.z _returnvalue))))
  (bind _returnvalue_5 (Math|Rotator|Delta(Rotator) _returnvalue_4 _returnvalue_3))
  (bind (_roll _pitch _yaw) (Math|Rotator|BreakRotator _returnvalue_5))
  (return _roll _pitch _yaw))

(fn CameraRange
  (params (PlayerIndex :type Integer))
  (bind _followcamera (Variables|Default|GetFollowCamera))
  (return (< (Class|KismetMathLibrary|DegAcos (Math|Vector|DotProduct (Math|Vector|GetForwardVector _followcamera) (Math|Vector|GetForwardVector (Math|Rotator|FindLookatRotation (Transformation|GetWorldLocation _followcamera) (Transformation|GetActorLocation (Game|GetPlayerCharacter PlayerIndex)))))) (Math|Float|MakeLiteralFloat 2e+01))))

(fn GetPlayerFindLookatRotation
  (params (PlayerID :type Integer))
  (bind _returnvalue (Transformation|GetActorLocation))
  (bind _returnvalue_2 (Game|GetPlayerCharacter PlayerID))
  (bind _returnvalue_3 (Transformation|GetActorLocation _returnvalue_2))
  (bind _returnvalue_4 (Math|Rotator|FindLookatRotation _returnvalue _returnvalue_3))
  (bind (_roll _pitch _yaw) (Math|Rotator|BreakRotator _returnvalue_4))
  (return _roll _pitch _yaw))

(fn IsAlive?
  (return (<= (Variables|ステータス|GetHealth) 0.0)))

(fn IsActorCheck
  (params (TagetActor :type Actor%20Object%20Reference))
  (return (== TagetActor (Variables|Actor|GetCharacterRef))))

(fn IsDistancetoCheck
  (params (PlayerID :type Integer))
  (return (<= (Transformation|GetDistanceTo (Game|GetPlayerCharacter PlayerID)) 5e+02)))