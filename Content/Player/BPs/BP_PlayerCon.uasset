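; Player controller that turns move, jump, attack, heavy attack, guard, avoid and deadly inputs into movement or message calls on the possessed pawn.
; An InputPossible flag gates these inputs, and attacks also check IsInDamage.
; Separate 2p inputs drive player character 1 directly, ignoring InputPossible.
; Attack2p uses a timer-based short/long press macro, but its release path is disconnected; SetControllerdPlayer possesses a given character.
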(event Custom|CustomEvent)

(event Custom|CustomEvent_1)

(event EventIsinInputPossible?
  (params (InputPossible :type Boolean))
  (Variables|Default|SetInput%20Possible InputPossible))

(event Input|ActionEvents|InputActionDeadly
  (params (Key :type Key%20Structure :default "None"))
  ;[0 1 0.7656] PlayerInput
  ;;[1 0.4922 0] 必殺
  (:Pressed
    (if (Variables|Default|GetInput%20Possible)
      (Class|BPPlayerInterface|DeadlyEvent(Message) (Pawn|GetControlledPawn)))))

(event Input|ActionEvents|InputActionAttack2p
  (params (Key :type Key%20Structure :default "None"))
  (bind _returnvalue (Game|GetPlayerCharacter 1))
  (:Pressed
    (if (not (Variables|/Game/Player/BPs/BP_PlayerCharacter.BP_PlayerCharacter_C|GetIs%20In%20Damage%20? (.AsBP%20Player%20Character (Utilities|Casting|CastToBP_PlayerCharacter (Game|GetPlayerCharacter 1)))))
      (Utilities|KeyEventSwitcher (delegate Custom|CustomEvent) (delegate Custom|CustomEvent_1) 3.0
        (:PostPressed
          (Class|BPPlayerInterface|PressedAttack(Message) _returnvalue))
        (:ShortPressReleased
          (Class|BPPlayerInterface|ShortPressedAttack(Message) _returnvalue))
        (:LongPressReleased
          (Class|BPPlayerInterface|LongPressedAttack(Message) _returnvalue))))))

(event Input|ActionEvents|InputActionGuard
  (params (Key :type Key%20Structure :default "None"))
  (bind _returnvalue (Pawn|GetControlledPawn))
  (bind _input_possible (Variables|Default|GetInput%20Possible))
  ;[0 1 0.7656] PlayerInput
  ;;[0.03125 0 1] ガード
  (:Pressed
    (if _input_possible
      (Class|BPPlayerInterface|OnGuard(Message) _returnvalue)))
  (:Released
    (if _input_possible
      (Class|BPPlayerInterface|OffGuard(Message) _returnvalue))))

(event Input|ActionEvents|InputActionAttack
  (params (Key :type Key%20Structure :default "None"))
  ;[0 1 0.7656] PlayerInput
  ;;[1 0 0.5156] 攻撃
  ;;;[1 0 0.8672] 通常攻撃
  (:Pressed
    (if (Variables|Default|GetInput%20Possible)
      (if (not (Variables|/Game/Player/BPs/BP_PlayerCharacter.BP_PlayerCharacter_C|GetIs%20In%20Damage%20? (.AsBP%20Player%20Character (Utilities|Casting|CastToBP_PlayerCharacter (Pawn|GetControlledPawn)))))
        (Class|BPPlayerInterface|PressedAttack(Message) (Pawn|GetControlledPawn))))))

(event Input|ActionEvents|InputActionHeavyAttack
  (params (Key :type Key%20Structure :default "None"))
  ;[0 1 0.7656] PlayerInput
  ;;[1 0 0.5156] 攻撃
  ;;;[0 1 0.9297] 強攻撃
  (:Pressed
    (if (Variables|Default|GetInput%20Possible)
      (if (not (Variables|/Game/Player/BPs/BP_PlayerCharacter.BP_PlayerCharacter_C|GetIs%20In%20Damage%20? (.AsBP%20Player%20Character (Utilities|Casting|CastToBP_PlayerCharacter (Pawn|GetControlledPawn)))))
        (Class|BPPlayerInterface|HeavyAttack(Message) (Pawn|GetControlledPawn))))))

(event Input|ActionEvents|InputActionJump
  (params (Key :type Key%20Structure :default "None"))
  (bind _returnvalue (Pawn|GetControlledPawn))
  (bind _input_possible (Variables|Default|GetInput%20Possible))
  ;[0 1 0.7656] PlayerInput
  ;;[0 0.3203 1] ジャンプ
  (:Pressed
    (if _input_possible
      (Class|BPPlayerInterface|JumpEvent(Message) _returnvalue)))
  (:Released
    (if _input_possible
      (Class|BPPlayerInterface|JumpStopEvent(Message) _returnvalue))))

(event Input|ActionEvents|InputActionJump2p
  (params (Key :type Key%20Structure :default "None"))
  (bind _returnvalue (Game|GetPlayerCharacter 1))
  (:Pressed
    (Class|BPPlayerInterface|JumpEvent(Message) _returnvalue))
  (:Released
    (Class|BPPlayerInterface|JumpStopEvent(Message) _returnvalue)))

(event Input|ActionEvents|InputActionAvoidance
  (params (Key :type Key%20Structure :default "None"))
  ;[0 1 0.7656] PlayerInput
  ;;[0.4766 0 1] 回避
  (:Pressed
    (if (Variables|Default|GetInput%20Possible)
      (Class|BPPlayerInterface|Avoid(Message) (Pawn|GetControlledPawn)))))

(event Input|AxisEvents|InputAxisMoveForward
  (params (AxisValue :type Float%20%28single-precision%29))
  ;[0 1 0.7656] PlayerInput
  ;;[0.3594 0 1] 移動
  (if (Variables|Default|GetInput%20Possible)
    (Pawn|Input|AddMovementInput (Pawn|GetControlledPawn) (Math|Vector|GetForwardVector (Math|Rotator|MakeRotator 0.0 0.0 (.Yaw (Math|Rotator|BreakRotator (Pawn|GetControlRotation (Pawn|GetControlledPawn) :!class /Script/Engine.Pawn))))) AxisValue false)))

(event Input|AxisEvents|InputAxisMoveRight
  (params (AxisValue :type Float%20%28single-precision%29))
  ;[0 1 0.7656] PlayerInput
  ;;[0.3594 0 1] 移動
  (if (Variables|Default|GetInput%20Possible)
    (Pawn|Input|AddMovementInput (Pawn|GetControlledPawn) (Math|Vector|GetRightVector (Math|Rotator|MakeRotator 0.0 0.0 (.Yaw (Math|Rotator|BreakRotator (Pawn|GetControlRotation (Pawn|GetControlledPawn) :!class /Script/Engine.Pawn))))) AxisValue false)))

(event Input|AxisEvents|InputAxisMoveForward2p
  (params (AxisValue :type Float%20%28single-precision%29))
  (Pawn|Input|AddMovementInput (Game|GetPlayerCharacter 1) (Math|Vector|GetForwardVector (Math|Rotator|MakeRotator 0.0 0.0 (.Yaw (Math|Rotator|BreakRotator (Pawn|GetControlRotation (Game|GetPlayerCharacter 1) :!class /Script/Engine.Pawn))))) AxisValue false))

(event Input|AxisEvents|InputAxisMoveRight2p
  (params (AxisValue :type Float%20%28single-precision%29))
  (Pawn|Input|AddMovementInput (Game|GetPlayerCharacter 1) (Math|Vector|GetRightVector (Math|Rotator|MakeRotator 0.0 0.0 (.Yaw (Math|Rotator|BreakRotator (Pawn|GetControlRotation (Game|GetPlayerCharacter 1) :!class /Script/Engine.Pawn))))) AxisValue false))

(fn ConstructionScript)

(fn SetControllerdPlayer
  (params (TagetCharacter :type BP%20Player%20Character%20Object%20Reference))
  (Pawn|Possess TagetCharacter)
  (return))