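; Match game mode that runs a local multiplayer fight and declares a winner by remaining health.
; BeginPlay creates a local player and tagged character at each BP_SpownPlayer point, links controllers through messages with input locked, plays music, then shows the start widget after a delay.
; Finish locks input again and shows the end widget for whoever has the most health, handling only Player 1 or 2 wins.
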(event Custom|Finish
  (bind _returnvalue (Game|GetPlayerController 0))
  (for (_array_element _array_index) (Variables|Default|GetPlayerCharacters)
    (Utilities|Array|Add (Variables|Default|GetPlayersHealth) (Variables|/Game/Player/BPs/BP_PlayerCharacter.BP_PlayerCharacter_C|GetHealth _array_element))
    (Class|BPPlayerConInterface|IsinInputPossible?(Message) (Game|GetPlayerController _array_index) false))
  (switch int (.IndexOfMaxValue (Math|Float|MaxOfFloatArray (Variables|Default|GetPlayersHealth)))
    (:0
      (bind _returnvalue_2 (UserInterface|CreateWidget "/Game/GameMode/Match/UI/BP_MatchEnd.BP_MatchEnd_C" _returnvalue))
      (Utilities|IsValid _returnvalue_2
        (:Is%20Valid
          (Rendering|Components|TextRender|SetText (Variables|/Game/GameMode/Match/UI/BP_MatchEnd.BP_MatchEnd_C|GetTextBlock_37 _returnvalue_2) "Player1 Win")
          (UserInterface|Viewport|AddtoViewport _returnvalue_2 0))))
    (:1
      (bind _returnvalue_3 (UserInterface|CreateWidget "/Game/GameMode/Match/UI/BP_MatchEnd.BP_MatchEnd_C" _returnvalue))
      (Utilities|IsValid _returnvalue_3
        (:Is%20Valid
          (Rendering|Components|TextRender|SetText (Variables|/Game/GameMode/Match/UI/BP_MatchEnd.BP_MatchEnd_C|GetTextBlock_37 _returnvalue_3) "Player2 Win")
          (UserInterface|Viewport|AddtoViewport _returnvalue_3 0))))))

(event EventBeginPlay
  (bind _outactors (Actor|GetAllActorsOfClass "/Game/Player/BPs/BP_SpownPlayer.BP_SpownPlayer_C"))
  (bind _output_get (Variables|Default|SetOut%20Actors _outactors))
  (for (_array_element _array_index) _output_get
    (Class|GameplayStatics|CreatePlayer _array_index)
    (bind _returnvalue (Game|SpawnActorfromClass "/Game/Player/BPs/BP_PlayerCharacter.BP_PlayerCharacter_C" (Math|Transform|MakeTransform (Transformation|GetActorLocation _array_element) (Transformation|GetActorRotation _array_element) "1,1,1") "Undefined" 0 0))
    (Class|BPPlayerConInterface|SetControllerdPlayer(Message) (Game|GetPlayerController _array_index) _returnvalue)
    (Class|BPPlayerConInterface|IsinInputPossible?(Message) (Game|GetPlayerController _array_index) false)
    (Utilities|Array|Add (Variables|Default|GetPlayerCharacters) _returnvalue)
    (Utilities|Array|Add (Variables|/Script/Engine.Actor|GetTags _returnvalue) (Utilities|Array|Get(acopy) (Variables|Default|GetPlayerTags) _array_index)))
  (Audio|PlaySound2D "/Game/Player/Sound/Alone_Cue.Alone_Cue" 1.0 1.0 0.0 0 0)
  (for _array_element_2 (Variables|Default|GetPlayerCharacters)
    (Class|BPPlayerInterface|SetControllerID(Message) _array_element_2)
    (Class|BPPlayerInterface|SetCharacterRef(Message) _array_element_2))
  (Utilities|FlowControl|Delay 1.0)
  (bind _returnvalue_2 (UserInterface|CreateWidget "/Game/GameMode/Match/UI/BP_MatchStart.BP_MatchStart_C" (Game|GetPlayerController 0)))
  (UserInterface|Viewport|AddtoViewport _returnvalue_2 0))

(event EventEndPlay
  (params (EndPlayReason :type EEndPlayReason%20Enum :default "Destroyed"))
  (Utilities|Array|Clear (Variables|Default|GetPlayerCharacters))
  (Utilities|Array|Clear (Variables|Default|GetPlayersHealth)))

(fn ConstructionScript)